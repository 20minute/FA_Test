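; BP_DialogTriggerComponent is an interaction component that starts a dialog when its owning BP_DialogTrigger actor is interacted with.
; On DoInteract it casts player controller 0 to BP_PlayerController and passes the owner's DialogueContext to that controller's dialog system component through TriggerDialog.
; It always allows interaction and reports a fixed interaction mode.
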(event `/Game/Core/Interactable/BPI_Interact.DoInteract`
  (bind _asbp_player_controller (cast `/Game/Core/Player/BP_PlayerController` (`GameplayStatics.GetPlayerController` 0)))
  (bind _asbp_dialog_trigger (cast `/Game/Core/Interactable/DialogTrigger/BP_DialogTrigger` (`self.GetOwner`)))
  (`/Game/Core/Dialog/BP_DialogSystemComponent.TriggerDialog` (`/Game/Core/Player/BP_PlayerController.BP_DialogSystemComponent` _asbp_player_controller) (`/Game/Core/Interactable/DialogTrigger/BP_DialogTrigger.DialogueContext` _asbp_dialog_trigger)))

(fn `CanInteract`
  (returns (Ouput :type Boolean))
  (return true))

(fn `GetInteractionMode`
  (returns (InteractionMode :type "/Game/Core/Interactable/EInteractionMode Enum"))
  (return "NewEnumerator5"))