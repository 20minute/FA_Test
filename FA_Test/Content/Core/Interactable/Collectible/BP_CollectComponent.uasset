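; BP_CollectComponent is an interaction component that lets a collectible item be picked up into the player's inventory.
; It caches the first player controller on BeginPlay, always allows interaction and reports a fixed interaction mode.
; On interact, it passes the owning BP_CollectibleItem's data to that controller's inventory component, then destroys the item actor.
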(event `self.ReceiveBeginPlay`
  (bind _asbp_player_controller (cast `/Game/Core/Player/BP_PlayerController` (`GameplayStatics.GetPlayerController` 0)))
  (set `self.As BP Player Controller` _asbp_player_controller))

(event `/Game/Core/Interactable/BPI_Interact.DoInteract`
  (bind _asbp_collectible_item (cast `/Game/Core/Interactable/Collectible/BP_CollectibleItem` (`self.GetOwner`)))
  (`/Game/Core/Inventory/BP_InventorySystemComponent.AddItemToInventory` (`/Game/Core/Player/BP_PlayerController.BP_InventorySystemComponent` (`self.As BP Player Controller`)) (`/Game/Core/Interactable/Collectible/BP_CollectibleItem.Data` _asbp_collectible_item))
  (`Actor.K2_DestroyActor` _asbp_collectible_item))

(fn `CanInteract`
  (returns (Ouput :type Boolean))
  (return true))

(fn `GetInteractionMode`
  (returns (InteractionMode :type "/Game/Core/Interactable/EInteractionMode Enum"))
  (return "NewEnumerator4"))