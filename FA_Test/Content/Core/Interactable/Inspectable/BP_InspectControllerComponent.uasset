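; Component that runs an inspect mode, letting the player rotate a copy of an interactable's static mesh with the mouse.
; Entering hides the pawn, disables its input, spawns a display actor ahead of the camera and switches view to a spawned inspect camera.
; Tick, toggled with the mode, turns mouse delta beyond a small threshold into rotation.
; Exiting restores the pawn and gameplay view, then destroys both spawned actors.
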(event `self.ReceiveBeginPlay`
  (bind _asbp_player_controller (cast `/Game/Core/Player/BP_PlayerController` (`GameplayStatics.GetPlayerController` 0)))
  (set `self.BP_PlayerController` _asbp_player_controller))

(event `self.ReceiveTick`
  (params (DeltaSeconds :type "Float (single-precision)"))
  (`self.RotateInspectedObject`))

(event `EnterInspectMode`
  (params (TargetActor :type "Actor Object Reference"))
  (`self.SetComponentTickEnabled` true)
  (set `self.TargetActor` TargetActor)
  (set `self.IsInspecting` true)
  (`self.TogglePlayer` true)
  (`self.ParepareInspection`)
  (`self.SpawnInspectedActor`)
  (`self.SpawnInspectedCamera`))

(event `ExitInspectMode`
  (`self.SetComponentTickEnabled` false)
  (if (`self.IsInspecting`)
    (set `self.TargetActor` null)
    (set `self.IsInspecting` false)
    (`self.TogglePlayer` false)
    (`self.Cleanup`)))

(fn `Cleanup`
  (bind _currentinspectedcamera (`self.CurrentInspectedCamera`))
  (bind _currentinspectedactor (`self.CurrentInspectedActor`))
  (`|ExecutionSequence`
    (:`then_0`
      (`PlayerController.SetViewTargetWithBlend` (`self.BP_PlayerController`) (`self.GameplayCamera`) 0.0 "VTBlend_Linear" 0.0 false))
    (:`then_1`
      (`/Engine/EditorBlueprintResources/StandardMacros.IsValid` _currentinspectedcamera
        (:`Is Valid`
          (`Actor.K2_DestroyActor` _currentinspectedcamera)
          (set `self.CurrentInspectedCamera` null))))
    (:`then_2`
      (`/Engine/EditorBlueprintResources/StandardMacros.IsValid` _currentinspectedactor
        (:`Is Valid`
          (`Actor.K2_DestroyActor` _currentinspectedactor)
          (set `self.CurrentInspectedActor` null))))
    (:`then_3`
      (set `self.InspectRotation` (struct)))))

(fn `ParepareInspection`
  (locals (CameraPosition :type "Vector Structure"))
  (bind _returnvalue (`GameplayStatics.GetPlayerCameraManager` 0))
  (bind _returnvalue_2 (`PlayerCameraManager.GetCameraRotation` _returnvalue))
  (bind _returnvalue_3 (`PlayerCameraManager.GetCameraLocation` _returnvalue))
  (bind _returnvalue_4 (`KismetMathLibrary.GetForwardVector` _returnvalue_2))
  (`|ExecutionSequence`
    (:`then_0`
      (`/Engine/EditorBlueprintResources/StandardMacros.IsValid` (`self.GameplayCamera`)
        (:`Is Not Valid`
          (set `self.GameplayCamera` (`Controller.GetViewTarget` (`self.BP_PlayerController`))))))
    (:`then_1`
      (set `self.InspectActorPosition` (+ (* _returnvalue_4 200.0) _returnvalue_3)))
    (:`then_2`
      (set `self.InspectCameraTransform` (`KismetMathLibrary.MakeTransform` (+ (* _returnvalue_4 1.0) _returnvalue_3) _returnvalue_2)))))

(fn `RotateInspectedObject`
  (bind _rotatespeed (`self.RotateSpeed`))
  (bind (_inspectrotation_roll _inspectrotation_pitch _inspectrotation_yaw) (`KismetMathLibrary.BreakRotator` (`self.InspectRotation`)))
  (bind (_deltax _deltay) (`PlayerController.GetInputMouseDelta` (`self.BP_PlayerController`)))
  (if (and (`self.IsInspecting`) (`KismetSystemLibrary.IsValid` (`self.CurrentInspectedActor`)))
    (if (or (> (`KismetMathLibrary.Abs` _deltax) 0.3) (> (`KismetMathLibrary.Abs` _deltay) 0.3))
      (bind _output_get (set `self.InspectRotation` (`KismetMathLibrary.MakeRotator` (+ _inspectrotation_roll (* _deltax _rotatespeed)) (- _inspectrotation_pitch (* _deltay _rotatespeed)) _inspectrotation_yaw)))
      (`Actor.K2_SetActorRelativeRotation` (`self.CurrentInspectedActor`) _output_get false false))))

(fn `SpawnInspectedActor`
  (bind _inspectactorposition (`self.InspectActorPosition`))
  (bind _asbp_interactable_base (cast `/Game/Core/Interactable/BP_InteractableBase` (`self.TargetActor`))
    (:`then`
      (if (`AIBlueprintHelperLibrary.IsValidAILocation` _inspectactorposition)
        (bind _returnvalue (`|SpawnActorFromClass` "/Game/Core/Interactable/Inspectable/BP_InspectDisplayActor.BP_InspectDisplayActor_C" (`KismetMathLibrary.MakeTransform` _inspectactorposition) "DontSpawnIfColliding" "MultiplyWithRoot" null null))
        (`/Game/Core/Interactable/Inspectable/BP_InspectDisplayActor.Init` _returnvalue (`StaticMeshComponent.StaticMesh` (`/Game/Core/Interactable/BP_InteractableBase.StaticMesh` _asbp_interactable_base)))
        (set `self.CurrentInspectedActor` _returnvalue)
        (else
          (`KismetSystemLibrary.PrintString` "Inspect Actor is not valid" true true (struct :`R` 1.0 :`G` 0.018015 :`A` 1.0)))))
    (:`CastFailed`
      (`KismetSystemLibrary.PrintString` "Target Actor is not Interactable" true true (struct :`R` 1.0 :`B` 0.075233 :`A` 1.0)))))

(fn `SpawnInspectedCamera`
  (bind _returnvalue (`|SpawnActorFromClass` "/Game/Core/Interactable/Inspectable/BP_InspectCamera.BP_InspectCamera_C" (`self.InspectCameraTransform`) "DontSpawnIfColliding" "MultiplyWithRoot" null null))
  (bind _output_get (set `self.CurrentInspectedCamera` _returnvalue))
  (`PlayerController.SetViewTargetWithBlend` (`self.BP_PlayerController`) _output_get 0.0 "VTBlend_Linear" 0.0 false))

(fn `TogglePlayer`
  (params (IsHiding :type Boolean))
  (bind _bp_playercontroller (`self.BP_PlayerController`))
  (bind _returnvalue (`Controller.K2_GetPawn` _bp_playercontroller))
  (`/Engine/EditorBlueprintResources/StandardMacros.IsValid` _bp_playercontroller
    (:`Is Valid`
      (if IsHiding
        (`Actor.SetActorHiddenInGame` _returnvalue true)
        (`Actor.DisableInput` _returnvalue _bp_playercontroller)
        (else
          (`Actor.SetActorHiddenInGame` _returnvalue false)
          (`Actor.EnableInput` _returnvalue _bp_playercontroller))))))