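; Player controller that handles first-level interaction input: world interaction, inspect-mode exit, inventory toggle and zoom.
; Each Tick, a Visibility line trace from the camera finds a BP_InteractableBase, caches it and toggles the interaction state of the cursor widget created at BeginPlay.
; Enhanced Input actions call the cached interactable, InspectController and inventory component, while zoom input is broadcast through WheelScrolled.
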(event `self.ReceiveBeginPlay`
  (bind _returnvalue (`|CreateWidget` "/Game/Core/UI/Cursor/WBP_Cursor.WBP_Cursor_C"))
  (`UserWidget.AddToViewport` _returnvalue 0)
  (set `self.WBP_Cursor` _returnvalue))

(event `self.ReceiveTick`
  (params (DeltaSeconds :type "Float (single-precision)"))
  (bind _returnvalue (`GameplayStatics.GetPlayerCameraManager` 0))
  (bind _returnvalue_2 (`PlayerCameraManager.GetCameraLocation` _returnvalue))
  (bind (_outhit _returnvalue_3) (`KismetSystemLibrary.LineTraceSingle` _returnvalue_2 (+ _returnvalue_2 (* (`KismetMathLibrary.GetForwardVector` (`PlayerCameraManager.GetCameraRotation` _returnvalue)) 1000)) "TraceTypeQuery1"))
  (if _returnvalue_3
    (bind _asbp_interactable_base (cast `/Game/Core/Interactable/BP_InteractableBase` (`.HitActor` (`GameplayStatics.BreakHitResult` _outhit)))
      (:`then`
        (set `self.CurrentInteractable` _asbp_interactable_base)
        (`/Game/Core/UI/Cursor/WBP_Cursor.ToggleInteraction` (`self.WBP_Cursor`) true))
      (:`CastFailed`
        (`/Game/Core/UI/Cursor/WBP_Cursor.ToggleInteraction` (`self.WBP_Cursor`) false :!label _label)
        (set `self.CurrentInteractable` null)))
    (else
      (goto _label))))

(event `EnhancedInput|/Game/Core/Input/Actions/IA_WorldInteract`
  (params (ActionValue :type Boolean) (ElapsedSeconds :type "Float (double-precision)") (TriggeredSeconds :type "Float (double-precision)") (InputAction :type "InputAction Object Reference" :default "/Game/Core/Input/Actions/IA_WorldInteract.IA_WorldInteract"))
  (bind _currentinteractable (`self.CurrentInteractable`))
  (:`Completed`
    (`/Engine/EditorBlueprintResources/StandardMacros.IsValid` _currentinteractable
      (:`Is Valid`
        (`/Game/Core/Interactable/BP_InteractableBase.DoInteract` _currentinteractable)))))

(event `EnhancedInput|/Game/Core/Input/Actions/IA_Cancel`
  (params (ActionValue :type Boolean) (ElapsedSeconds :type "Float (double-precision)") (TriggeredSeconds :type "Float (double-precision)") (InputAction :type "InputAction Object Reference" :default "/Game/Core/Input/Actions/IA_Cancel.IA_Cancel"))
  (:`Canceled`
    (`/Game/Core/Interactable/Inspectable/BP_InspectControllerComponent.ExitInspectMode` (`self.InspectController`))))

(event `EnhancedInput|/Game/Core/Input/Actions/IA_Inventory`
  (params (ActionValue :type Boolean) (ElapsedSeconds :type "Float (double-precision)") (TriggeredSeconds :type "Float (double-precision)") (InputAction :type "InputAction Object Reference" :default "/Game/Core/Input/Actions/IA_Inventory.IA_Inventory"))
  (:`Completed`
    (`/Game/Core/Inventory/BP_InventorySystemComponent.ToggleInventoryUI` (`self.BP_InventorySystemComponent`))))

(event `EnhancedInput|/Game/Core/Input/Actions/IA_Zoom`
  (params (ActionValue :type "Float (double-precision)") (ElapsedSeconds :type "Float (double-precision)") (TriggeredSeconds :type "Float (double-precision)") (InputAction :type "InputAction Object Reference" :default "/Game/Core/Input/Actions/IA_Zoom.IA_Zoom"))
  (:`Triggered`
    (`self.WheelScrolled` ActionValue)))

(fn `UserConstructionScript`)