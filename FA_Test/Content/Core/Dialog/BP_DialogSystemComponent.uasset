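; BP_DialogSystemComponent is a component that shows and dismisses the game's dialog box.
; TriggerDialog creates a DialogBoxClass widget, adds it to the viewport, initializes it with the given dialog context, then shows the cursor and switches player 0 to UI-only input focused on it.
; OnDialogEnd removes the widget, hides the cursor and restores game-only input, with IsShowingDialog tracking the state.
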(event `TriggerDialog`
  (params (DialogContext :type "/Game/Core/Dialog/FDialogueEntry Structure"))
  (bind _returnvalue (`GameplayStatics.GetPlayerController` 0))
  (bind _returnvalue_2 (`|CreateWidget` (`self.DialogBoxClass`)))
  (`UserWidget.AddToViewport` _returnvalue_2 0)
  (bind _output_get (set `self.DialogBoxRef` _returnvalue_2))
  (`/Game/Core/Dialog/WBP_DialogueBox.Init` _output_get DialogContext)
  (set `PlayerController.bShowMouseCursor` true _returnvalue)
  (`WidgetBlueprintLibrary.SetInputMode_UIOnlyEx` _returnvalue (`self.DialogBoxRef`))
  (set `self.IsShowingDialog` true))

(event `OnDialogEnd`
  (bind _returnvalue (`GameplayStatics.GetPlayerController` 0))
  (bind _dialogboxref (`self.DialogBoxRef`))
  (`/Engine/EditorBlueprintResources/StandardMacros.IsValid` _dialogboxref
    (:`Is Valid`
      (`Widget.RemoveFromParent` _dialogboxref))
    (:`Is Not Valid`
      _))
  (set `self.DialogBoxRef` null)
  (set `PlayerController.bShowMouseCursor` false _returnvalue)
  (`WidgetBlueprintLibrary.SetInputMode_GameOnly` _returnvalue)
  (set `self.IsShowingDialog` false))