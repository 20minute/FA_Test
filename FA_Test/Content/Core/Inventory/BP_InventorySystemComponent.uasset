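; Inventory component that stores collected items and manages the inventory screen.
; Added items go into an array that is pushed to the widget, which is created on show and removed on hide.
; Showing the screen enables the cursor and Game and UI input mode while disabling pawn input; hiding reverses this.
; The widget's forget-note event drives a filter that keeps only one item type, apparently 3D items, then refreshes the display.
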(event `self.ReceiveBeginPlay`)

(fn `AddItemToInventory`
  (params (CollectibleItem :type "/Game/Core/Inventory/FInventoryItem Structure"))
  (`KismetArrayLibrary.Array_Add` (`self.InventoryItems`) CollectibleItem)
  ; Update UI if open
  (if (`self.IsShowingUI`)
    (`self.UpdateInventoryUI`)))

(fn `HideInventoryUI`
  (bind _returnvalue (`GameplayStatics.GetPlayerController` 0))
  (bind _inventoryuiref (`self.InventoryUIRef`))
  (clear `/Game/Core/Inventory/UI/WBP_Inventory.OnForgetNoteButtonClicked` _inventoryuiref)
  (`Widget.RemoveFromParent` _inventoryuiref)
  (set `PlayerController.bShowMouseCursor` false _returnvalue)
  (`WidgetBlueprintLibrary.SetInputMode_GameOnly` _returnvalue)
  (`Actor.EnableInput` (`Controller.K2_GetPawn` _returnvalue) _returnvalue)
  (set `self.IsShowingUI` false))

(fn `OnForgetButtonClicked`
  (locals (`3DItems` :type "Array of /Game/Core/Inventory/FInventoryItem Structure"))
  (bind _inventoryuiref (`self.InventoryUIRef`))
  (`|ExecutionSequence`
    (:`then_0`
      (for _array_element (`self.InventoryItems`)
        (if (`|EnumEquality` (`.Type_15_934C87864652198533E23EA097BE4F3B` (break `/Game/Core/Inventory/FInventoryItem` _array_element)) "NewEnumerator1")
          (`KismetArrayLibrary.Array_Add` (`local.3DItems`) _array_element)))
      (set `self.InventoryItems` (`local.3DItems`)))
    (:`then_1`
      (`/Engine/EditorBlueprintResources/StandardMacros.IsValid` _inventoryuiref
        (:`Is Valid`
          (`/Game/Core/Inventory/UI/WBP_Inventory.UpdateInventory` _inventoryuiref (`self.InventoryItems`)))))))

(fn `ShowInventoryUI`
  (bind _returnvalue (`GameplayStatics.GetPlayerController` 0))
  (bind _returnvalue_2 (`|CreateWidget` (`self.InventoryUIClass`)))
  (bind _output_get (set `self.InventoryUIRef` _returnvalue_2))
  (add `/Game/Core/Inventory/UI/WBP_Inventory.OnForgetNoteButtonClicked` _output_get (`|CreateDelegate` :!event `OnForgetButtonClicked`))
  (`UserWidget.AddToViewport` _output_get 0)
  (set `PlayerController.bShowMouseCursor` true _returnvalue)
  (`WidgetBlueprintLibrary.SetInputMode_GameAndUIEx` _returnvalue (`self.InventoryUIRef`))
  (`Actor.DisableInput` (`Controller.K2_GetPawn` _returnvalue) _returnvalue)
  (`self.UpdateInventoryUI`)
  (set `self.IsShowingUI` true))

(fn `ToggleInventoryUI`
  (if (`self.IsShowingUI`)
    (`self.HideInventoryUI`)
    (else
      (`self.ShowInventoryUI`))))

(fn `UpdateInventoryUI`
  (`/Game/Core/Inventory/UI/WBP_Inventory.UpdateInventory` (`self.InventoryUIRef`) (`self.InventoryItems`)))